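; Actor component for environment music that adds UI-sound flagging and volume fading on top of its parent's behavior.
; On BeginPlay, if IsUISound is set, it marks the audio components under the owner's root as UI sounds.
; SetNewVolume either applies a target volume immediately or flags a fade.
; Tick then moves Volume toward the target at a constant rate, clearing the flag once reached.
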(event `self.ReceiveBeginPlay`
  (`parent.ReceiveBeginPlay`)
  (`self.SetUISound`))

(event `self.ReceiveTick`
  (params (DeltaSeconds :type "Float (single-precision)"))
  (`parent.ReceiveTick` DeltaSeconds)
  (`self.FadeVolume` DeltaSeconds))

(fn `SetNewVolume`
  (params (TargetVolume :type "Float (double-precision)") (`Fade?` :type Boolean))
  (bind _output_get (set `self.TarVolume` TargetVolume))
  (bind _output_get_2 (set `self.FadeVolumeFlag` `Fade?`))
  (if (not _output_get_2)
    (set `self.Volume` _output_get)))

(fn `SetUISound`
  (if (`self.IsUISound`)
    (for _array_element (`SceneComponent.GetChildrenComponents` (`Actor.RootComponent` (`self.GetOwner`)) true)
      (bind _asaudio_component (cast `AudioComponent` _array_element))
      (set `AudioComponent.bIsUISound` true _asaudio_component))))