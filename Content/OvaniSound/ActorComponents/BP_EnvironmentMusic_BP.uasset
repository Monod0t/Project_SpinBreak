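; Actor component that plays queued environment music as MetaSounds, with crossfades, skipping and adjustable intensity.
; Parallel arrays queue each song's lengths, variant and fade time, and the last entry repeats until replaced or skipped.
; Tick compares wall-clock time against the song's length minus reverb tail, then alternates between two runtime-created AudioComponents.
; Tick also crossfades their volumes and blends the Intensity parameter on both, while LoopNum selects the clip variant.
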(event `self.ReceiveBeginPlay`
  (bind _returnvalue (`self.GetOwner`))
  ;[0.151 0.1486 0] Blueprint Init
  (bind _returnvalue_2 (`|AddComponentByClass` :`self` _returnvalue :`Class` "/Script/Engine.AudioComponent"))
  (`AudioComponent.Stop` _returnvalue_2)
  (set `self.AudioSource1` _returnvalue_2)
  (bind _returnvalue_3 (`|AddComponentByClass` :`self` _returnvalue :`Class` "/Script/Engine.AudioComponent"))
  (`AudioComponent.Stop` _returnvalue_3)
  (set `self.AudioSource2` _returnvalue_3))

(event `self.ReceiveTick`
  (params (DeltaSeconds :type "Float (single-precision)"))
  (bind _volume (`self.Volume`))
  (bind (_year _month _day _hour _minute _second _millisecond) (`KismetMathLibrary.BreakDateTime` (`KismetMathLibrary.Now`)))
  (bind (_year_2 _month_2 _day_2 _hour_2 _minute_2 _second_2 _millisecond_2) (`KismetMathLibrary.BreakDateTime` (`self.PlayStartTime`)))
  (bind _returnvalue (/ (`self.CurTransitionTime`) (`self.Transition Length`)))
  (bind _returnvalue_2 (- (`|GetArrayItem` (`self.PendingSounds_MainLengths`)) (`|GetArrayItem` (`self.PendingSounds_TailLengths`))))
  (bind _returnvalue_3 (- (+ (`KismetMathLibrary.Conv_IntToDouble` (+ (* (+ (* (+ (* _day 24) _hour) 60) _minute) 60) _second)) (/ (`KismetMathLibrary.Conv_IntToDouble` _millisecond) 1000.0)) (+ (`KismetMathLibrary.Conv_IntToDouble` (+ (* (+ (* (+ (* _day_2 24) _hour_2) 60) _minute_2) 60) _second_2)) (/ (`KismetMathLibrary.Conv_IntToDouble` _millisecond_2) 1000.0))))
  (`|ExecutionSequence`
    (:`then_0`
      ;[0.04321 0.1171 0.8333] Song Playback
      (if (!= (`KismetArrayLibrary.Array_Length` (`self.PendingSounds`)) 0)
        (if (!= (`|GetArrayItem` (`self.PendingSounds`)) (`self.LastSound`))
          (`self.(Internal Use Only) Next Song`) ; Trigger a Refresh to Start Playback.
          (else
            (`|ExecutionSequence`
              (:`then_0`
                (if (and (< (`self.Last Tick Time (Accurate)`) _returnvalue_2) (> _returnvalue_3 _returnvalue_2))
                  (`self.(Internal Use Only) Next Song`) ; Trigger Next song or Loop.
                ))
              (:`then_1`
                (set `self.Last Tick Time (Accurate)` _returnvalue_3) ; Timestamp the last Milisecond of playback.
              ))))
        (else
          (`self.(Internal Use Only) Next Song`) ; No song? Refresh to Stop playback.
        )))
    (:`then_1`
      ;[0.001194 0.02604 0.000668] Song Crossfading
      (`/Engine/EditorBlueprintResources/StandardMacros.IsValid` (`self.PlayingSource`)
        (:`Is Valid`
          (`/Engine/EditorBlueprintResources/StandardMacros.IsValid` (`self.FadingSource`)
            (:`Is Valid`
              (if (== (`self.CurTransitionTime`) -1.0)
                (`AudioComponent.SetVolumeMultiplier` (`self.FadingSource`) _volume :!label _label)
                (`AudioComponent.SetVolumeMultiplier` (`self.PlayingSource`) _volume)
                (elif (> (`self.CurTransitionTime`) 0.0)
                  (bind _output_get (set `self.CurTransitionTime` (- (stale _output_get) DeltaSeconds))) ; Countdown the Transition Time
                  (`AudioComponent.SetVolumeMultiplier` (`self.FadingSource`) (* (`self.Volume`) _returnvalue)) ; Fade Current song volume in by Transition%
                  (`AudioComponent.SetVolumeMultiplier` (`self.PlayingSource`) (* (- 1.0 _returnvalue) (`self.Volume`))) ; Fade Last Song volume out by Transition%
                  (elif (!= (`|GetArrayItem` (`self.PendingSounds`)) (`self.LastSound`))
                    (goto _label)))))))))
    (:`then_2`
      ;[0.2812 0 0] Intensity Fading
      (bind _output_get_2 (set `self.IntensityFadeTime` (+ (stale _output_get_2) DeltaSeconds))) ; Track how much time is passed since an intensity fade was started
      (bind _returnvalue_4 (`KismetMathLibrary.FClamp` (`KismetMathLibrary.SafeDivide` _output_get_2 (`self.IntensityBlendTime`))))
      (bind _returnvalue_5 (`KismetMathLibrary.Lerp` (`self.Intensity Fade Start`) (`self.Intensity`) _returnvalue_4))
      (`AudioParameterControllerInterface.SetFloatParameter` (`self.AudioSource1`) "Intensity" _returnvalue_5)
      (`AudioParameterControllerInterface.SetFloatParameter` (`self.AudioSource2`) "Intensity" _returnvalue_5)
      (if (>= _returnvalue_4 1.0)
        (set `self.Intensity Fade Start` (`self.Intensity`)) ; Record the Current Intensity as the\nStartPoint for the next Intensity Fade
      ))))

(event `(Internal Use Only) Swap & Play`
  (params (`Meta Sound` :type "MetaSoundSource Object Reference"))
  (bind _audiosource1 (`self.AudioSource1`))
  (bind _audiosource2 (`self.AudioSource2`))
  (set `self.PlayStartTime` (`KismetMathLibrary.Now`))
  (bind _output_get (set `self.CurrentSource` (== (`self.CurrentSource`) false)))
  (if _output_get
    (`/Engine/EditorBlueprintResources/StandardMacros.IsValid` `Meta Sound`
      (:`Is Valid`
        (`AudioComponent.SetSound` _audiosource1 `Meta Sound`)
        (set `self.LastSound` `Meta Sound`))
      (:`Is Not Valid`
        _))
    (`AudioComponent.Play` _audiosource1 0.0)
    (set `self.PlayingSource` _audiosource1)
    (set `self.FadingSource` _audiosource2)
    (else
      (`/Engine/EditorBlueprintResources/StandardMacros.IsValid` `Meta Sound`
        (:`Is Valid`
          (`AudioComponent.SetSound` _audiosource2 `Meta Sound`)
          (set `self.LastSound` `Meta Sound`))
        (:`Is Not Valid`
          _))
      (`AudioComponent.Play` _audiosource2 0.0)
      (set `self.PlayingSource` _audiosource2)
      (set `self.FadingSource` _audiosource1))))

(event `(Internal Use Only) Next Song`
  (bind _pendingsounds_loopnum (`self.PendingSounds_LoopNum`))
  (bind _pendingsounds_fadetime (`self.PendingSounds_FadeTime`))
  (bind _pendingsounds (`self.PendingSounds`))
  (bind _returnvalue (`KismetArrayLibrary.Array_Length` (`self.PendingSounds`)))
  (bind _output (`|GetArrayItem` _pendingsounds_fadetime))
  (if (!= _returnvalue 0)
    (if (!= (`self.LastSound`) null)
      (if (not (== _returnvalue 1))
        (`KismetArrayLibrary.Array_Remove` _pendingsounds)
        (`KismetArrayLibrary.Array_Remove` (`self.PendingSounds_MainLengths`))
        (`KismetArrayLibrary.Array_Remove` (`self.PendingSounds_TailLengths`))
        (`KismetArrayLibrary.Array_Remove` _pendingsounds_loopnum)
        (`KismetArrayLibrary.Array_Remove` _pendingsounds_fadetime))
      (`self.(Internal Use Only) Swap & Play` (`|GetArrayItem` _pendingsounds) :!label _label)
      (`AudioComponent.SetFloatParameter` (`self.PlayingSource`) "LoopNum" (/ (`KismetMathLibrary.Conv_IntToDouble` (`|GetArrayItem` _pendingsounds_loopnum)) 2.0))
      (bind _output_get (set `self.CurTransitionTime` (`KismetMathLibrary.SelectFloat` 0.025 _output (== _output 0.0))))
      (set `self.Transition Length` _output_get)
      (else
        (`|ExecutionSequence`
          (:`then_0`
            (goto _label))
          (:`then_1`
            (bind _output_get_2 (set `self.CurTransitionTime` -1.0))
            (set `self.Transition Length` _output_get_2)))))
    (else
      (`self.(Internal Use Only) Swap & Play` null)
      (`AudioComponent.SetSound` (`self.PlayingSource`) null))))

(fn `Play Looping Song`
  (params (Song :type "MetaSoundSource Object Reference") (`Clip Length` :type "Float (double-precision)") (`Reverb Tail Length` :type "Float (double-precision)") (`Clip Alts Selection` :type Integer) (`Play Now / Clear Queue` :type Boolean) (`Play Now Fade Time` :type "Float (double-precision)"))
  (if `Play Now / Clear Queue`
    (set `self.PendingSounds` (`|MakeArray` Song))
    (set `self.PendingSounds_MainLengths` (`|MakeArray` `Clip Length`))
    (set `self.PendingSounds_TailLengths` (`|MakeArray` `Reverb Tail Length`))
    (set `self.PendingSounds_LoopNum` (`|MakeArray` `Clip Alts Selection`))
    (set `self.PendingSounds_FadeTime` (`|MakeArray` `Play Now Fade Time`))
    (else
      (`KismetArrayLibrary.Array_Add` (`self.PendingSounds`) Song)
      (`KismetArrayLibrary.Array_Add` (`self.PendingSounds_MainLengths`) `Clip Length`)
      (`KismetArrayLibrary.Array_Add` (`self.PendingSounds_TailLengths`) `Reverb Tail Length`)
      (`KismetArrayLibrary.Array_Add` (`self.PendingSounds_LoopNum`) `Clip Alts Selection`)
      (`KismetArrayLibrary.Array_Add` (`self.PendingSounds_FadeTime`) (`KismetMathLibrary.SelectFloat` (`KismetMathLibrary.SelectFloat` 0.025 `Play Now Fade Time` (== `Play Now Fade Time` 0.0)) -1.0 `Play Now / Clear Queue`)))))

(fn `Set Intensity 0-1`
  (params (Intensity :type "Float (double-precision)") (`Blend Time` :type "Float (double-precision)"))
  (set `self.Intensity` (* Intensity 2.0))
  (set `self.IntensityBlendTime` (`KismetMathLibrary.SelectFloat` 0.0001 `Blend Time` (== `Blend Time` 0.0)))
  (set `self.IntensityFadeTime` 0.0))

(fn `Skip Songs`
  (params (Amount :type Integer) (TransitionTime :type "Float (double-precision)"))
  (bind _returnvalue (- Amount 1))
  (if (>= _returnvalue (`KismetArrayLibrary.Array_Length` (`self.PendingSounds`)))
    (`KismetArrayLibrary.Array_Clear` (`self.PendingSounds`))
    (`KismetArrayLibrary.Array_Clear` (`self.PendingSounds_MainLengths`))
    (`KismetArrayLibrary.Array_Clear` (`self.PendingSounds_TailLengths`))
    (`KismetArrayLibrary.Array_Clear` (`self.PendingSounds_LoopNum`))
    (`KismetArrayLibrary.Array_Clear` (`self.PendingSounds_FadeTime`))
    (else
      (for _ (range (+ _returnvalue 1))
        (`KismetArrayLibrary.Array_Remove` (`self.PendingSounds`))
        (`KismetArrayLibrary.Array_Remove` (`self.PendingSounds_MainLengths`))
        (`KismetArrayLibrary.Array_Remove` (`self.PendingSounds_TailLengths`))
        (`KismetArrayLibrary.Array_Remove` (`self.PendingSounds_LoopNum`))
        (`KismetArrayLibrary.Array_Remove` (`self.PendingSounds_FadeTime`)))
      (`KismetArrayLibrary.Array_Set` (`self.PendingSounds_FadeTime`) 0 (`KismetMathLibrary.SelectFloat` 0.001 TransitionTime (== TransitionTime 0.0)))
      (`self.(Internal Use Only) Next Song`))))