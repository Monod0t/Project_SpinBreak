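; Cube enemy pawn that detects BP_PlayerSphere through a range sphere and moves via FloatingPawnMovement while detection lasts.
; Tick applies manual gravity, gated by a downward line trace, and HuntPlayer, which steers from the cube toward its own actor location rather than the stored TargetPlayer.
; BeginPlay passes the damage range to the damage component, but hit damage and death binding are unwired; direction and visual functions are empty.
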(event `self.ReceiveBeginPlay`
  (bind _bp_damage_component (`self.BP_Damage_Component`))
  (set `/Game/SpinBreak/Blueprints/Components/BP_Damage_Component.DamageMin` (`self.DamageMin`) _bp_damage_component)
  (set `/Game/SpinBreak/Blueprints/Components/BP_Damage_Component.DamageMax` (`self.DamageMax`) _bp_damage_component))

(event `OnDeathCS`
  (`SceneComponent.SetVisibility` (`self.Cube`) false false))

(event `self.ReceiveTick`
  (params (DeltaSeconds :type "Float (single-precision)"))
  (`self.HandleGravity` DeltaSeconds)
  (`self.HuntPlayer`))

(event `self.Cube.OnComponentHit`
  (params (HitComponent :type "PrimitiveComponent Object Reference") (OtherActor :type "Actor Object Reference") (OtherComp :type "PrimitiveComponent Object Reference") (NormalImpulse :type "Vector Structure") (Hit :type "HitResult Structure (by ref)")))

(event `self.SphereRange.OnComponentBeginOverlap`
  (params (OverlappedComponent :type "PrimitiveComponent Object Reference") (OtherActor :type "Actor Object Reference") (OtherComp :type "PrimitiveComponent Object Reference") (OtherBodyIndex :type Integer) (bFromSweep :type Boolean) (SweepResult :type "HitResult Structure (by ref)"))
  (bind _asbp_player_sphere (cast `/Game/SpinBreak/Blueprints/Player/BP_PlayerSphere` OtherActor))
  (set `self.TargetPlayer` _asbp_player_sphere)
  (set `self.DetectedPlayer` true))

(event `self.SphereRange.OnComponentEndOverlap`
  (params (OverlappedComponent :type "PrimitiveComponent Object Reference") (OtherActor :type "Actor Object Reference") (OtherComp :type "PrimitiveComponent Object Reference") (OtherBodyIndex :type Integer))
  (bind _asbp_player_sphere (cast `/Game/SpinBreak/Blueprints/Player/BP_PlayerSphere` OtherActor))
  (set `self.TargetPlayer` _asbp_player_sphere)
  (set `self.DetectedPlayer` false))

(fn `HandleDirection`
  (locals (NewLocalVar :type "Transform Structure")))

(fn `HandleGravity`
  (params (`Delta Seconds` :type "Float (double-precision)"))
  (bind _floatingpawnmovement (`self.FloatingPawnMovement`))
  (bind _floatingpawnmovement_2 (`self.FloatingPawnMovement`))
  (bind (_velocity_x _velocity_y _velocity_z) (`KismetMathLibrary.BreakVector` (`MovementComponent.Velocity` _floatingpawnmovement)))
  (bind _grounddetected (`self.GroundDetection`))
  (if _grounddetected
    (set `MovementComponent.Velocity` (`KismetMathLibrary.MakeVector` _velocity_x _velocity_y (`KismetMathLibrary.FMax` 0.0 _velocity_z)) _floatingpawnmovement)
    (else
      (set `MovementComponent.Velocity` (+ (`MovementComponent.Velocity` _floatingpawnmovement_2) (* (* (* `Delta Seconds` (`self.Gravity`)) (`KismetMathLibrary.MakeVector` 0.0 0.0 -1.0)) (`KismetMathLibrary.Conv_DoubleToVector` 500.0))) _floatingpawnmovement_2))))

(fn `HandleVisuals`
  (params (`Delta Seconds` :type "Float (double-precision)")))

(fn `HuntPlayer`
  (bind (_returnvalue_x _returnvalue_y) (`KismetMathLibrary.BreakVector` (`KismetMathLibrary.GetDirectionUnitVector` (`SceneComponent.K2_GetComponentLocation` (`self.Cube`)) (`self.K2_GetActorLocation`))))
  (if (`self.DetectedPlayer`)
    (`PawnMovementComponent.AddInputVector` (`self.FloatingPawnMovement`) (`KismetMathLibrary.MakeVector` _returnvalue_x _returnvalue_y) false)))

(fn `UserConstructionScript`)

(fn `VisualizeBallMotions`
  (params (`Delta Seconds` :type "Float (double-precision)"))
  (locals (NumOfSpins :type Integer :default 3)))