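; Player pawn for SpinBreak: a mouse-aimed rolling ball with jump, parry hop and chargeable spin shot, which rams health-component actors for speed-scaled damage.
; While alive, Tick runs custom gravity, ability timers with ground-trace charge refills, screen-space cursor aiming, FloatingPawnMovement input and procedural mesh spin.
; Spin shots temporarily override speed tuning, restored from cached base values.
; Health, armor and death events start CSS feedback; death also hides the sphere.
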(event `self.ReceiveBeginPlay`
  (bind _bp_health_component (`self.BP_Health_Component`))
  (bind _bp_damage_component (`self.BP_Damage_Component`))
  (`self.InitializeSpeedVariables`)
  (set `self.CurChargesAvailable` (`self.MaxChargesAvailable`))
  (set `/Game/SpinBreak/Blueprints/Components/BP_Damage_Component.DamageMin` (`self.DamageMin`) _bp_damage_component)
  (set `/Game/SpinBreak/Blueprints/Components/BP_Damage_Component.DamageMax` (`self.DamageMax`) _bp_damage_component)
  (add `/Game/SpinBreak/Blueprints/Components/BP_Health_Component.OnHealthChange` _bp_health_component (delegate `OnHpDamageCS`))
  (add `/Game/SpinBreak/Blueprints/Components/BP_Health_Component.OnArmorChange` _bp_health_component (delegate `OnArmorDmgCS`))
  (add `/Game/SpinBreak/Blueprints/Components/BP_Health_Component.OnDeath` _bp_health_component (delegate `OnDeathCS`)))

(event `self.ReceiveTick`
  (params (DeltaSeconds :type "Float (single-precision)"))
  (if (`KismetMathLibrary.Conv_IntToBool` (`/Game/SpinBreak/Blueprints/Components/BP_Health_Component.CurHealth` (`self.BP_Health_Component`)))
    (`self.HandleGravity` DeltaSeconds)
    (`self.HandleAbilities` DeltaSeconds)
    (`self.HandleDirection`)
    (`self.HandleSpeed`)
    (`self.HandleVisuals` DeltaSeconds)))

(event `self.Sphere.OnComponentHit`
  (params (HitComponent :type "PrimitiveComponent Object Reference") (OtherActor :type "Actor Object Reference") (OtherComp :type "PrimitiveComponent Object Reference") (NormalImpulse :type "Vector Structure") (Hit :type "HitResult Structure (by ref)"))
  (bind _returnvalue (`self.GetComponentByClass` OtherActor "/Game/SpinBreak/Blueprints/Components/BP_Health_Component.BP_Health_Component_C"))
  (bind _returnvalue_2 (`KismetMathLibrary.VSize` (`MovementComponent.Velocity` (`self.FloatingPawnMovement`))))
  (if (`KismetSystemLibrary.IsValid` _returnvalue)
    (if (>= _returnvalue_2 (* (`self.MaxSpeed`) (`self.MinSpeedPercentage`)))
      (bind _calcdmg (`/Game/SpinBreak/Blueprints/Components/BP_Damage_Component.CalcPercentageDamage` (`self.BP_Damage_Component`) (/ _returnvalue_2 (`self.MaxSpeed`))))
      (`/Game/SpinBreak/Blueprints/Components/BP_Health_Component.TakeDmg` _returnvalue _calcdmg))))

(event `OnHpDamageCS`
  (`CameraShakeSourceComponent.Start` (`self.CSS-OnHpDmg`)))

(event `OnArmorDmgCS`
  (`CameraShakeSourceComponent.Start` (`self.CSS-OnArmorDmg`)))

(event `TriggerJump_Event`)

(event `OnDeathCS`
  (`CameraShakeSourceComponent.Start` (`self.CSS-OnDealth`))
  (`SceneComponent.SetVisibility` (`self.Sphere`) false false))

(event `TriggerParry_Event`)

(event `TriggerShoot_Event`)

(event `TriggerRecoil_Event`)

(fn `ActivateCharging`
  (if (not (or (`self.Charging`) (`self.Shooting`) (<= (`self.CurChargesAvailable`) 0)))
    (set `self.CurChargeTime` 0.0)
    (set `self.Charging` true)
    (set `self.ChargeStart` true)
    (set `self.ChargeReady` false)
    (set `FloatingPawnMovement.Deceleration` (`self.BrakeSpeed`) (`self.FloatingPawnMovement`))
    (`GameplayStatics.PlaySound2D` "/Game/Assets/Sfx/Sfx_Charge_Cue.Sfx_Charge_Cue" 1.0 1.0 0.0 null null)))

(fn `ActivateJump`
  (bind _curjumpcharges (`self.CurJumpCharges`))
  (if (`KismetMathLibrary.Conv_IntToBool` _curjumpcharges)
    (`/Engine/EditorBlueprintResources/StandardMacros.DecrementInt` _curjumpcharges
      (:`  `
        (if (`self.Driving`)
          (set `MovementComponent.Velocity` (`self.RedirectCurVelocity` (`self.RawDirection`) (`self.JumpSpd`)) (`self.FloatingPawnMovement`))
          (else
            (set `MovementComponent.Velocity` (`self.ApplyVertVelocity` (`self.JumpSpd`)) (`self.FloatingPawnMovement`))))
        (`GameplayStatics.PlaySound2D` "/Game/Assets/Sfx/Sfx_Jump_Cue.Sfx_Jump_Cue" 1.0 1.0 0.0 null null)
        (set `self.Grounded` false)))))

(fn `ActivateParry`
  (bind _curparrycharges (`self.CurParryCharges`))
  (bind _floatingpawnmovement (`self.FloatingPawnMovement`))
  (if (and (`KismetMathLibrary.Conv_IntToBool` _curparrycharges) (<= (`self.CurParryCooldown`) 0.0))
    (`/Engine/EditorBlueprintResources/StandardMacros.DecrementInt` _curparrycharges
      (:`  `
        (set `self.CurParryDuration` (`self.MaxParryDuration`))
        (set `self.CurParryCooldown` (`self.MaxParryCooldown`))
        (set `self.Parrying` true)
        (set `self.ParryStart` true)
        (if (`self.Driving`)
          (set `MovementComponent.Velocity` (`self.RedirectCurVelocity` (`self.RawDirection`) (`self.ParryHopSpd`)) _floatingpawnmovement)
          (else
            (set `MovementComponent.Velocity` (`self.ApplyVertVelocity` (`self.ParryHopSpd`)) _floatingpawnmovement)))
        (`GameplayStatics.PlaySound2D` "/Game/Assets/Sfx/Sfx_Parry_Cue.Sfx_Parry_Cue" 1.0 1.0 0.0 null null)
        (set `self.Grounded` false)))))

(fn `ActivateShooting`
  (bind (_calcmaxspd _calcaccel _calcdecel _calcbrakespd) (`self.CalculateShootingSpeeds`))
  (if (not (`self.Shooting`))
    (`self.FinishCharging`)
    (`self.UpdateSpeedVariables` _calcmaxspd _calcaccel _calcdecel _calcbrakespd)
    (set `MovementComponent.Velocity` (`self.CalculateSpinShotVelocity`) (`self.FloatingPawnMovement`))
    (set `self.CurSpinShotDuration` (- (`self.CurChargeTime`) (`self.MinChargeTime`)))
    (`GameplayStatics.PlaySound2D` "/Game/Assets/Sfx/Sfx_Shoot_Cue.Sfx_Shoot_Cue" 1.0 1.0 0.0 null null)
    (set `self.Shooting` true)))

(fn `ApplyPulse`)

(fn `FinishCharging`
  (set `self.Charging` false)
  (set `self.ChargeStart` false)
  (set `self.ChargeReady` false))

(fn `FinishShooting`
  (set `self.Charging` false)
  (set `self.ChargeReady` false)
  (set `self.Shooting` false)
  (`self.ResetSpeedVariables` true))

(fn `HandleAbilities`
  (params (`Delta Seconds` :type "Float (double-precision)"))
  (`self.TickParryCooldown` `Delta Seconds`)
  (`self.TickCharging` `Delta Seconds`)
  (`self.TickSpinShotDuration` `Delta Seconds`)
  (`self.FadeTurningBoost` `Delta Seconds`)
  (bind _grounddetected (`self.GroundDetection`))
  (if _grounddetected
    (`/Engine/EditorBlueprintResources/StandardMacros.DoOnce` false :!label _label
      (:`Completed`
        (set `self.CurJumpCharges` (`self.MaxJumpCharges`))
        (set `self.CurParryCharges` (`self.MaxParryCharges`))))
    (else
      (goto _label :!via `Reset`))))

(fn `HandleCameraControls`)

(fn `HandleDirection`
  (locals (NewLocalVar :type "Transform Structure"))
  (bind _returnvalue (* (`PlayerController.ProjectWorldLocationToScreen` (`GameplayStatics.GetPlayerController` 0) (`SceneComponent.K2_GetComponentLocation` (`self.Sphere`)) true) (`KismetMathLibrary.MultiplyMultiply_FloatFloat` (`WidgetLayoutLibrary.GetViewportScale`) -1.0)))
  (bind _returnvalue_2 (`WidgetLayoutLibrary.GetMousePositionOnViewport`))
  (bind _output_get (set `self.RawDirection` (`KismetMathLibrary.GetRotated2D` (`KismetMathLibrary.Normal2D` (- _returnvalue_2 _returnvalue)) 90.0)))
  (if (>= (`KismetMathLibrary.Distance2D` _returnvalue_2 _returnvalue) (`self.ControlRange`))
    (set `self.CalDirection` _output_get)
    (else
      (set `self.CalDirection` (0.0 0.0))))
  (return))

(fn `HandleGravity`
  (params (`Delta Seconds` :type "Float (double-precision)"))
  (bind _floatingpawnmovement (`self.FloatingPawnMovement`))
  (bind _floatingpawnmovement_2 (`self.FloatingPawnMovement`))
  (bind (_velocity_x _velocity_y _velocity_z) (`KismetMathLibrary.BreakVector` (`MovementComponent.Velocity` _floatingpawnmovement)))
  (if (`self.Grounded`)
    (set `MovementComponent.Velocity` (`KismetMathLibrary.MakeVector` _velocity_x _velocity_y (`KismetMathLibrary.FMax` 0.0 _velocity_z)) _floatingpawnmovement)
    (else
      (set `MovementComponent.Velocity` (+ (`MovementComponent.Velocity` _floatingpawnmovement_2) (* (* (* `Delta Seconds` (`self.Gravity`)) (`KismetMathLibrary.MakeVector` 0.0 0.0 -1.0)) (`KismetMathLibrary.Conv_DoubleToVector` 500.0))) _floatingpawnmovement_2))))

(fn `HandleSpeed`
  (if (`self.Grounded`)
    ; Decelerate
    (set `FloatingPawnMovement.Deceleration` (`self.Deceleration`) (`self.FloatingPawnMovement`))
    (if (or (`self.Shooting`) (`self.Charging`))
      (if (`self.Charging`)
        ; Charging Shot
        (if (`self.ChargeStart`)
          (set `self.ChargeStart` false)
          (elif (and (`self.Grounded`) (< (`self.CurChargeTime`) (`self.MaxChargeTime`)))
            (if (< (`self.CurChargeTime`) (`self.MinChargeTime`))
              (`PawnMovementComponent.AddInputVector` (`self.FloatingPawnMovement`) (`KismetMathLibrary.Conv_Vector2DToVector` (* (`KismetMathLibrary.Negated2D` (`self.RawDirection`)) (`self.MaxChargeKickback`))) false)
              (else
                (set `self.ChargeReady` true)))
            (else
              (`self.ActivateShooting`))))
        (else
          ; Spin Shot
          (`PawnMovementComponent.AddInputVector` (`self.FloatingPawnMovement`) (`KismetMathLibrary.Conv_Vector2DToVector` (`self.RawDirection`)) false)))
      (elif (`self.Driving`)
        ; Drive
        (bind _output_get (set `self.CurDirection` (`self.CalDirection`)))
        (`PawnMovementComponent.AddInputVector` (`self.FloatingPawnMovement`) (`KismetMathLibrary.Conv_Vector2DToVector` _output_get) false)
        (elif (`self.Braking`)
          ; Brake
          (set `FloatingPawnMovement.Deceleration` (`self.BrakeSpeed`) (`self.FloatingPawnMovement`)))))
    (else
      ; Maintain Speed while Airborne
      (set `FloatingPawnMovement.Deceleration` 0.0 (`self.FloatingPawnMovement`)))))

(fn `HandleVisuals`
  (params (`Delta Seconds` :type "Float (double-precision)"))
  (`self.VisualizeBallMotions` `Delta Seconds`))

(fn `InitializeSpeedVariables`
  (bind _output_get (set `self.BaseMaxSpeed` (`self.MaxSpeed`)))
  (bind _output_get_2 (set `self.BaseAcceleration` (`self.Acceleration`)))
  (bind _output_get_3 (set `self.BaseDeceleration` (`self.Deceleration`)))
  (bind _output_get_4 (set `self.BaseBrakeSpeed` (`self.BrakeSpeed`)))
  (bind _output_get_5 (set `self.BaseTurningBoost` (`self.TurningBoost`)))
  (`self.UpdateSpeedVariables` _output_get _output_get_2 _output_get_3 _output_get_4 _output_get_5))

(fn `Interrupt`)

(fn `ResetSpeedVariables`
  (params (ResetMaxSpd :type Boolean :default true) (ResetAccel :type Boolean :default true) (ResetDecel :type Boolean :default true) (ResetBrakeSpd :type Boolean :default true) (ResetTurningBoost :type Boolean :default true))
  (if ResetMaxSpd
    (bind _output_get (set `self.MaxSpeed` (`self.BaseMaxSpeed`)))
    (set `FloatingPawnMovement.MaxSpeed` _output_get (`self.FloatingPawnMovement`)))
  (if ResetAccel
    (bind _output_get_2 (set `self.Acceleration` (`self.BaseAcceleration`)))
    (set `FloatingPawnMovement.Acceleration` _output_get_2 (`self.FloatingPawnMovement`)))
  (if ResetDecel
    (bind _output_get_3 (set `self.Deceleration` (`self.BaseDeceleration`)))
    (set `FloatingPawnMovement.Deceleration` _output_get_3 (`self.FloatingPawnMovement`)))
  (if ResetBrakeSpd
    (set `self.BrakeSpeed` (`self.BaseBrakeSpeed`)))
  (if ResetTurningBoost
    (set `self.TurningBoost` (`self.BaseTurningBoost`))))

(fn `UpdateSpeedVariables`
  (params (NewMaxSpd :type "Float (double-precision)") (NewAccel :type "Float (double-precision)") (NewDecel :type "Float (double-precision)") (NewBrakeSpd :type "Float (double-precision)") (NewTurningBoost :type "Float (double-precision)"))
  (if (not (<= NewMaxSpd 0.0))
    (bind _output_get (set `self.MaxSpeed` (`KismetMathLibrary.FMax` 0.0 NewMaxSpd)))
    (set `FloatingPawnMovement.MaxSpeed` _output_get (`self.FloatingPawnMovement`)))
  (if (not (<= NewAccel 0.0))
    (bind _output_get_2 (set `self.Acceleration` (`KismetMathLibrary.FMax` 0.0 NewAccel)))
    (set `FloatingPawnMovement.Acceleration` _output_get_2 (`self.FloatingPawnMovement`)))
  (if (not (<= NewDecel 0.0))
    (bind _output_get_3 (set `self.Deceleration` (`KismetMathLibrary.FMax` 0.0 NewDecel)))
    (set `FloatingPawnMovement.Deceleration` _output_get_3 (`self.FloatingPawnMovement`)))
  (if (not (<= NewBrakeSpd 0.0))
    (set `self.BrakeSpeed` (`KismetMathLibrary.FMax` 0.0 NewBrakeSpd))
    (if (not (< NewTurningBoost 0.0))
      (bind _output_get_4 (set `self.TurningBoost` (`KismetMathLibrary.FMax` 0.0 NewTurningBoost)))
      (set `FloatingPawnMovement.TurningBoost` _output_get_4 (`self.FloatingPawnMovement`)))))

(fn `UserConstructionScript`)

(fn `VisualizeBallMotions`
  (params (`Delta Seconds` :type "Float (double-precision)"))
  (locals (NumOfSpins :type Integer :default 3))
  (bind _spheremesh (`self.SphereMesh`))
  (bind _maxspinshotmulti (`self.MaxSpinShotMulti`))
  (bind _returnvalue (/ 360.0 (`self.MaxParryDuration`)))
  (bind (_returnvalue_x _returnvalue_y) (`KismetMathLibrary.BreakVector` (* (`MovementComponent.Velocity` (`self.FloatingPawnMovement`)) `Delta Seconds`)))
  (bind (_returnvalue_x_2 _returnvalue_y_2) (`KismetMathLibrary.BreakVector` (* (* (`self.RawDirection`) (`MovementComponent.GetMaxSpeed` (`self.FloatingPawnMovement`))) `Delta Seconds`)))
  (if (`self.Parrying`)
    (if (`self.ParryStart`)
      ; Start of Parry
      (set `self.ParryStart` false)
      (bind _result (`/Engine/EditorBlueprintResources/StandardMacros.NegateFloat` _returnvalue)
        (:`  `
          (bind _output_get (set `self.CurParrySpinSpd` (* (`KismetMathLibrary.SelectFloat` _returnvalue _result (`KismetMathLibrary.RandomBool`)) (`local.NumOfSpins`)))))))
    (bind _returnvalue_2 (* _output_get `Delta Seconds`))
    ; Apply Parry Spin
    (`SceneComponent.K2_AddWorldRotation` _spheremesh (`KismetMathLibrary.MakeRotator` 0.0 0.0 _returnvalue_2) false false)
    (return)
    (elif (and true (`self.Charging`))
      ; Rotate Charging Spin Shot
      (bind _result_2 (`/Engine/EditorBlueprintResources/StandardMacros.NegateFloat` _returnvalue_x_2)
        (:`  `
          (`SceneComponent.K2_AddWorldRotation` _spheremesh (`KismetMathLibrary.MakeRotator` (* _returnvalue_y_2 _maxspinshotmulti) (* _result_2 _maxspinshotmulti)) false false)))
      (else
        (set `self.CurParrySpinSpd` (`KismetMathLibrary.FInterpTo` (`self.CurParrySpinSpd`) 0.0 `Delta Seconds` 5.0))
        ; Rotate Rolling using Velocity
        (bind _result_3 (`/Engine/EditorBlueprintResources/StandardMacros.NegateFloat` _returnvalue_x)
          (:`  `
            (`SceneComponent.K2_AddWorldRotation` _spheremesh (`KismetMathLibrary.MakeRotator` _returnvalue_y _result_3 _returnvalue_2) false false)
            (return)))))))