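; Player controller for SpinBreak that turns Enhanced Input into actions on the controlled BP_PlayerSphere.
; On BeginPlay it adds the mapping context and caches the sphere and game manager.
; Drive, brake, jump and parry forward to the sphere, while the P key triggers pause through the manager.
; A short Drive tap opens a timed window where pressing again starts charging; release shoots if the charge is ready.
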(event `self.ReceiveBeginPlay`
  (bind _returnvalue (subsystem `EnhancedInputLocalPlayerSubsystem`))
  ;[0.05098 0.05098 0.05098] Add Mapping Context
  (`/Engine/EditorBlueprintResources/StandardMacros.IsValid` _returnvalue
    (:`Is Valid`
      (`EnhancedInputSubsystemInterface.AddMappingContext` _returnvalue "/Game/SpinBreak/Input/IMC_SpinBreak.IMC_SpinBreak" 0 (struct))
      (bind _asbp_player_sphere (cast `/Game/SpinBreak/Blueprints/Player/BP_PlayerSphere` (`self.K2_GetPawn`))
        (:`then`
          (set `self.PlayerSphere` _asbp_player_sphere)
          (bind _returnvalue_2 (`GameplayStatics.GetActorOfClass` "/Game/SpinBreak/Blueprints/BP_GameManager.BP_GameManager_C"))
          (set `self.GameManager` _returnvalue_2))
        (:`CastFailed`
          (`KismetSystemLibrary.PrintString` "FAILED TO FIND PLAYER SPHERE!"))))
    (:`Is Not Valid`
      (`KismetSystemLibrary.PrintString` "FAILED VALIDATION"))))

(event `EnhancedInput|/Game/SpinBreak/Input/Actions/IA_Drive`
  (params (ActionValue :type Boolean) (ElapsedSeconds :type "Float (double-precision)") (TriggeredSeconds :type "Float (double-precision)") (InputAction :type "InputAction Object Reference" :default "/Game/SpinBreak/Input/Actions/IA_Drive.IA_Drive"))
  (bind _quicktapthreshold (`self.QuickTapThreshold`))
  (bind _playersphere (`self.PlayerSphere`))
  (:`Started`
    (set `/Game/SpinBreak/Blueprints/Player/BP_PlayerSphere.Driving` true _playersphere)
    (if (`self.QuickTapped`)
      (`/Game/SpinBreak/Blueprints/Player/BP_PlayerSphere.ActivateCharging` _playersphere)))
  (:`Completed`
    (set `/Game/SpinBreak/Blueprints/Player/BP_PlayerSphere.Driving` false _playersphere)
    (if (`/Game/SpinBreak/Blueprints/Player/BP_PlayerSphere.Charging` _playersphere)
      (if (`/Game/SpinBreak/Blueprints/Player/BP_PlayerSphere.ChargeReady` _playersphere)
        (`/Game/SpinBreak/Blueprints/Player/BP_PlayerSphere.ActivateShooting` _playersphere)
        (else
          (`/Game/SpinBreak/Blueprints/Player/BP_PlayerSphere.FinishCharging` _playersphere :!label _label)
          (if (>= ElapsedSeconds _quicktapthreshold)
            (if (stale _output_get)
              (set `self.QuickTapped` false :!label _label_2))
            (else
              (`|ExecutionSequence`
                (:`then_0`
                  (bind _output_get (set `self.QuickTapped` true)))
                (:`then_1`
                  (`KismetSystemLibrary.Delay` _quicktapthreshold)
                  (goto _label_2)))))))
      (else
        (goto _label)))))

(event `EnhancedInput|/Game/SpinBreak/Input/Actions/IA_Brake`
  (params (ActionValue :type Boolean) (ElapsedSeconds :type "Float (double-precision)") (TriggeredSeconds :type "Float (double-precision)") (InputAction :type "InputAction Object Reference" :default "/Game/SpinBreak/Input/Actions/IA_Brake.IA_Brake"))
  (:`Started`
    (set `/Game/SpinBreak/Blueprints/Player/BP_PlayerSphere.Braking` true (`self.PlayerSphere`)))
  (:`Completed`
    (set `/Game/SpinBreak/Blueprints/Player/BP_PlayerSphere.Braking` false (`self.PlayerSphere`))))

(event `EnhancedInput|/Game/SpinBreak/Input/Actions/IA_Jump`
  (params (ActionValue :type Boolean) (ElapsedSeconds :type "Float (double-precision)") (TriggeredSeconds :type "Float (double-precision)") (InputAction :type "InputAction Object Reference" :default "/Game/SpinBreak/Input/Actions/IA_Jump.IA_Jump"))
  (:`Started`
    (`/Game/SpinBreak/Blueprints/Player/BP_PlayerSphere.ActivateJump` (`self.PlayerSphere`))))

(event `EnhancedInput|/Game/SpinBreak/Input/Actions/IA_Parry`
  (params (ActionValue :type Boolean) (ElapsedSeconds :type "Float (double-precision)") (TriggeredSeconds :type "Float (double-precision)") (InputAction :type "InputAction Object Reference" :default "/Game/SpinBreak/Input/Actions/IA_Parry.IA_Parry"))
  (:`Started`
    (`/Game/SpinBreak/Blueprints/Player/BP_PlayerSphere.ActivateParry` (`self.PlayerSphere`))))

(event `EnhancedInput|/Game/SpinBreak/Input/Actions/IA_Charge`
  (params (ActionValue :type Boolean) (ElapsedSeconds :type "Float (double-precision)") (TriggeredSeconds :type "Float (double-precision)") (InputAction :type "InputAction Object Reference" :default "/Game/SpinBreak/Input/Actions/IA_Charge.IA_Charge")))

(event `Key|P` :paused true
  (params (Key :type "Key Structure"))
  (:`Pressed`
    (`/Game/SpinBreak/Blueprints/BP_GameManager.TriggerPause_Event` (`self.GameManager`))))

(fn `UserConstructionScript`)