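; Game manager for SpinBreak that runs the round flow as an enum state machine, advanced on Tick from initialization through timed gameplay to upgrade draft or game over.
; BeginPlay starts looping music, creates player info and pause widgets, and binds player death to RoundFailed.
; Timer expiry also fails the round, muting music, while RoundWin changes music intensity.
; State entry logic only prints the state; random objective selection exists but is never called here.
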(event `self.ReceiveBeginPlay`
  (`self.InitializeMusicPlayer`)
  (`self.InstatiateWidgets` (delegate `RoundFailed`))
  (`self.ChangeGameState` "NewEnumerator0"))

(event `self.ReceiveTick`
  (params (DeltaSeconds :type "Float (single-precision)"))
  (switch `/Game/SpinBreak/Enums/EStateMachine` (`self.CurState`)
    (:`NewEnumerator0`
      (`KismetSystemLibrary.Delay` (`self.RoundStartDelay`))
      (`self.ChangeGameState` "NewEnumerator5"))
    (:`NewEnumerator5`
      (`KismetSystemLibrary.Delay` (`self.RoundStartDelay`))
      (`self.ChangeGameState` "NewEnumerator1"))
    (:`NewEnumerator1`
      (`self.TickRoundTimer` DeltaSeconds))
    (:`NewEnumerator2`
      (if (not (`self.FailedRunFlag`))
        (`self.ChangeGameState` "NewEnumerator3")
        (else
          (`self.ChangeGameState` "NewEnumerator4"))))))

(event `TriggerPause_Event`
  (`/Game/SpinBreak/Widgets/WB_PauseMenu.TogglePause` (`self.PauseMenu`)))

(event `RoundStart`)

(event `RoundWin`
  (`/Game/OvaniSound/ActorComponents/BP_EnvironmentMusic_BP.Set Intensity 0-1` (`self.BP_EnvironmentMusic_BP_Modified`) 0.5 0.5)
  (`self.ChangeGameState` "NewEnumerator2"))

(event `RoundFailed`
  (set `self.FailedRunFlag` true)
  (`/Game/OvaniSound/ActorComponents/BP_EnvironmentMusic_BP_Modified.SetNewVolume` (`self.BP_EnvironmentMusic_BP_Modified`) 0.0 false)
  (`self.ChangeGameState` "NewEnumerator2"))

(fn `AdjustMusicPlayer`
  (params (Volume :type "Float (double-precision)") (VolumeBlendTime :type "Float (double-precision)") (Intensity :type "Float (double-precision)") (IntensityBlendTime :type "Float (double-precision)"))
  (`/Game/OvaniSound/ActorComponents/BP_EnvironmentMusic_BP_Modified.SetNewVolume` (`self.BP_EnvironmentMusic_BP_Modified`) Volume (!= 0.0 (`KismetMathLibrary.FMax` 0.0 VolumeBlendTime)))
  (`/Game/OvaniSound/ActorComponents/BP_EnvironmentMusic_BP.Set Intensity 0-1` (`self.BP_EnvironmentMusic_BP_Modified`) Intensity IntensityBlendTime)
  (return))

(fn `ChangeGameState`
  (params (`New State` :type "/Game/SpinBreak/Enums/EStateMachine Enum" :default "NewEnumerator0"))
  (bind _output_get (set `self.CurState` `New State`))
  (switch `/Game/SpinBreak/Enums/EStateMachine` _output_get
    (:`NewEnumerator0`
      _)
    (:`NewEnumerator5`
      _)
    (:`NewEnumerator1`
      _)
    (:`NewEnumerator2`
      _)
    (:`NewEnumerator3`
      _)
    (:`NewEnumerator4`
      _))
  (`KismetSystemLibrary.PrintString` (`|GetEnumeratorNameAsString` _output_get)))

(fn `GenerateRoundObjective`
  (bind _roundobjectivelist (`self.RoundObjectiveList`))
  (if (`KismetArrayLibrary.Array_IsNotEmpty` _roundobjectivelist)
    (set `self.CurRoundObjective` (`KismetArrayLibrary.Array_Random` _roundobjectivelist))
    (else
      (set `self.CurRoundObjective` "NewEnumerator0")))
  (return))

(fn `InitializeMusicPlayer`
  (`/Game/OvaniSound/ActorComponents/BP_EnvironmentMusic_BP.Play Looping Song` (`self.BP_EnvironmentMusic_BP_Modified`) (`self.StartingMusic`) 85.0 1.19 0 false 0.0)
  (`self.AdjustMusicPlayer` (`self.StartingVolume`) 0.0 (`self.StartingIntensity`)))

(fn `InstatiateWidgets`
  (params (Delegate :type "Delegate (by ref)"))
  (bind _returnvalue (`GameplayStatics.GetActorOfClass` "/Game/SpinBreak/Blueprints/Player/BP_PlayerSphere.BP_PlayerSphere_C"))
  (bind _output_get (set `self.PlayerSphere` _returnvalue))
  (add `/Game/SpinBreak/Blueprints/Components/BP_Health_Component.OnDeath` (`/Game/SpinBreak/Blueprints/Player/BP_PlayerSphere.BP_Health_Component` _output_get) Delegate)
  (bind _returnvalue_2 (`|CreateWidget` "/Game/SpinBreak/Widgets/WB_PlayerInfo.WB_PlayerInfo_C" (`GameplayStatics.GetPlayerController` 0)))
  (bind _output_get_2 (set `self.PlayerInfo` _returnvalue_2))
  (`UserWidget.AddToViewport` _output_get_2 0)
  (bind _returnvalue_3 (`|CreateWidget` "/Game/SpinBreak/Widgets/WB_PauseMenu.WB_PauseMenu_C" (`GameplayStatics.GetPlayerController` 0)))
  (bind _output_get_3 (set `self.PauseMenu` _returnvalue_3))
  (`UserWidget.AddToViewport` _output_get_3 9))

(fn `UserConstructionScript`)