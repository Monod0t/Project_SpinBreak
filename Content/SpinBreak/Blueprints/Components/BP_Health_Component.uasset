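; Health component that tracks armor and health for its owner, resetting both to max on BeginPlay.
; Incoming damage, blocked by Unkillable or Invulnerable, drains armor before spilling into health, with armor change signalled only on fully absorbed hits.
; Change and death calls notify listeners, with 2D sounds for armor hits, health hits and death.
; A settable or stackable invulnerability duration counts down on Tick; DeathCheck is an empty stub.
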(event `self.ReceiveBeginPlay`
  (`self.ResetValues`))

(event `self.ReceiveTick`
  (params (DeltaSeconds :type "Float (single-precision)"))
  (`self.TickInvulnerability` DeltaSeconds))

(event `TakeHealthDmg_Event`
  (params (InflictedDmg :type Integer))
  (`self.CalculateDmgTaken` InflictedDmg))

(event `OnDeath_Event`
  (`GameplayStatics.PlaySound2D` (`self.DeathSfx`) 1.0 1.0 0.0 null null))

(fn `CalculateDmgTaken`
  (params (IncomingDmg :type Integer))
  (locals (RemainingDmg :type Integer))
  (if (not (`self.Unkillable`))
    (if (not (`self.Invulnerable`))
      (bind _output_get (set `local.RemainingDmg` IncomingDmg))
      (if (`KismetMathLibrary.Conv_IntToBool` _output_get)
        (bind (_remainingtarget _remainingdmg) (`self.CalculateRemainingValue` (`self.CurArmor`) _output_get))
        (set `self.CurArmor` _remainingtarget)
        (bind _output_get_2 (set `local.RemainingDmg` _remainingdmg))
        (if (not (`KismetMathLibrary.Conv_IntToBool` _output_get_2))
          (`self.OnArmorChange`)
          (`GameplayStatics.PlaySound2D` (`self.ArmorDmgSfx`) 1.0 1.0 0.0 null null)
          (else
            (bind _remainingtarget_2 (`self.CalculateRemainingValue` (`self.CurHealth`) _output_get_2))
            (bind _output_get_3 (set `self.CurHealth` _remainingtarget_2))
            (`self.OnHealthChange`)
            (if (<= _output_get_3 0)
              (`self.OnDeath`)
              (else
                (`GameplayStatics.PlaySound2D` (`self.HealthDmgSfx`) 1.0 1.0 0.0 null null)))))
        (else
          (`KismetSystemLibrary.PrintString` "NO INITIAL DMG INFLICTED")))
      (else
        (`KismetSystemLibrary.PrintString` "TARGET NOT KILLABLE")))
    (else
      (`KismetSystemLibrary.PrintString` "TARGET NOT KILLABLE"))))

(fn `CalculateRemainingValue`
  (params (TargetValue :type Integer) (IncomingDmg :type Integer))
  (returns (RemainingTarget :type Integer) (RemainingDmg :type Integer))
  (locals (NewLocalVar :type Integer) (NewLocalVar_0 :type Integer))
  (bind _returnvalue (- TargetValue IncomingDmg))
  (if (>= _returnvalue 0)
    (return _returnvalue 0)
    (else
      (return 0 (`KismetMathLibrary.Abs_Int` _returnvalue)))))

(fn `DeathCheck`)

(fn `ResetValues`
  (set `self.CurHealth` (`self.MaxHealth`))
  (`self.OnHealthChange`)
  (set `self.CurArmor` (`self.MaxArmor`))
  (`self.OnArmorChange`))

(fn `SetInvulnerability`
  (params (InvincibleDuration :type "Float (double-precision)") (Override :type Boolean))
  (if Override
    (set `self.InvulnerableDuration` InvincibleDuration)
    (else
      (set `self.InvulnerableDuration` (+ (`self.InvulnerableDuration`) InvincibleDuration)))))