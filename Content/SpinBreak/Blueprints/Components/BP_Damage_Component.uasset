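; BP_Damage_Component is a component that computes integer damage values from its DamageMin and DamageMax range.
; CalcRandomDamage returns a random integer within that range.
; CalcPercentageDamage clamps a 0–1 fraction, maps it linearly onto the range, then rounds and clamps the result.
; It only calculates values; its event graph has no active logic and it does not apply damage.
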(fn `CalcPercentageDamage`
  (params (Percentage :type "Float (double-precision)" :default 1.0))
  (returns (CalcDmg :type Integer))
  (return (`KismetMathLibrary.Clamp` (`KismetMathLibrary.Round` (`KismetMathLibrary.MapRangeClamped` (`KismetMathLibrary.FClamp` Percentage) 0.0 1.0 (`KismetMathLibrary.Conv_IntToDouble` (`self.DamageMin`)) (`KismetMathLibrary.Conv_IntToDouble` (`self.DamageMax`)))) (`self.DamageMin`) (`self.DamageMax`))))

(fn `CalcRandomDamage`
  (returns (CalcDmg :type Integer))
  (return (`KismetMathLibrary.RandomIntegerInRange` (`self.DamageMin`) (`self.DamageMax`))))